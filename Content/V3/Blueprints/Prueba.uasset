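; Test actor (Prueba) with a ball component (Bola), a box trigger and a particle system.
; While Presionadam is true, Tick draws a debug Visibility trace from the ball toward its forward vector scaled out, not offset by location, and ignores the result.
; Any overlap on the box destroys the ball, begins particle trails and removes the box.
; Debug prints mark each stage; no movement is implemented.
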(event `self.ReceiveTick`
  (params (DeltaSeconds :type "Float (single-precision)"))
  (bind _bola (`self.bola`))
  (if (`self.presionadam`)
    (`KismetSystemLibrary.PrintString` "Lleego a prueba")
    (`KismetSystemLibrary.LineTraceSingle` :`Start` (`SceneComponent.K2_GetComponentLocation` _bola) :`End` (* (`SceneComponent.GetForwardVector` _bola) 5000.0) :`TraceChannel` "TraceTypeQuery1" :`DrawDebugType` "ForDuration")
    (`KismetSystemLibrary.PrintString` "Mover")))

(event `self.Box.OnComponentBeginOverlap`
  (params (OverlappedComponent :type "PrimitiveComponent Object Reference") (OtherActor :type "Actor Object Reference") (OtherComp :type "PrimitiveComponent Object Reference") (OtherBodyIndex :type Integer) (bFromSweep :type Boolean) (SweepResult :type "HitResult Structure (by ref)"))
  (`KismetSystemLibrary.PrintString` "Colision")
  (`ActorComponent.K2_DestroyComponent` (`self.bola`))
  (`ParticleSystemComponent.BeginTrails` (`self.ParticleSystem`) "None" "None" "ETrailWidthMode_FromCentre" 0.0)
  (`ActorComponent.K2_DestroyComponent` (`self.Box`)))

(fn `UserConstructionScript`)