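; Health power-up: a spinning heart that adds 10 to the Vida of an overlapping Character_gatoBase.
; On pickup, which requires the heart to be visible, it plays a sound, prints a debug string and hides the heart.
; Tick rotates the heart and uses a Delay with the AparecerVida flag to make it visible roughly every five seconds, independent of when it was collected.
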(event `self.ReceiveBeginPlay`)

(event `self.ReceiveTick`
  (params (DeltaSeconds :type "Float (single-precision)"))
  (bind _aparecer_vida (`self.aparecer_vida`))
  (`|ExecutionSequence`
    (:`then_0`
      (if (not _aparecer_vida)
        (`KismetSystemLibrary.Delay` 5.0)
        (set `self.aparecer_vida` true)))
    (:`then_1`
      (if _aparecer_vida
        (`SceneComponent.SetVisibility` (`self.corazoncito`) true false)
        (set `self.aparecer_vida` false)))
    (:`then_2`
      (`SceneComponent.K2_AddLocalRotation` (`self.corazoncito`) (`KismetMathLibrary.MakeRotator` 0.0 0.0 (* DeltaSeconds (`self.rotar_corazon`))) false false))))

(event `self.corazon.OnComponentBeginOverlap`
  (params (OverlappedComponent :type "PrimitiveComponent Object Reference") (OtherActor :type "Actor Object Reference") (OtherComp :type "PrimitiveComponent Object Reference") (OtherBodyIndex :type Integer) (bFromSweep :type Boolean) (SweepResult :type "HitResult Structure (by ref)"))
  (if (`SceneComponent.IsVisible` (`self.corazoncito`))
    (bind _ascharacter_gato_base (cast `/Game/V3/Modelos_OBJ/Personaje/Base/BP_gatoBase/Character_gatoBase` OtherActor))
    (set `/Game/V3/Modelos_OBJ/Personaje/Base/BP_gatoBase/Character_gatoBase.vida` (+ (`/Game/V3/Modelos_OBJ/Personaje/Base/BP_gatoBase/Character_gatoBase.vida` _ascharacter_gato_base) 10.0) _ascharacter_gato_base)
    (`KismetSystemLibrary.PrintString` "Eentro")
    (`GameplayStatics.PlaySound2D` "/Game/V3/SonidosyMusica/Sonidos/power_up.power_up" 1.0 1.0 0.0 null null)
    (`SceneComponent.SetVisibility` (`self.corazoncito`) false false)))

(fn `UserConstructionScript`)