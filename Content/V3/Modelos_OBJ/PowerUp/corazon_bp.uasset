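; Heart power-up pickup that restores health (Vida) to the cat character, Character_gatoBase.
; Tick spins the Corazon component around its yaw axis at a frame-rate-independent speed set by Rotation.
; Overlaps on Corazon or Sphere share one path that casts to the cat, adds a fixed amount of Vida and sets VidaTomadaCor.
; It then prints a debug string, plays a 2D sound and destroys itself.
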(event `self.ReceiveTick`
  (params (DeltaSeconds :type "Float (single-precision)"))
  (`SceneComponent.K2_AddLocalRotation` (`self.corazon`) (`KismetMathLibrary.MakeRotator` 0.0 0.0 (* DeltaSeconds (`self.rotation`))) false false))

(event `self.corazon.OnComponentBeginOverlap`
  (params (OverlappedComponent :type "PrimitiveComponent Object Reference") (OtherActor :type "Actor Object Reference") (OtherComp :type "PrimitiveComponent Object Reference") (OtherBodyIndex :type Integer) (bFromSweep :type Boolean) (SweepResult :type "HitResult Structure (by ref)"))
  (bind _ascharacter_gato_base (cast `/Game/V3/Modelos_OBJ/Personaje/Base/BP_gatoBase/Character_gatoBase` (stale `self.Sphere.OnComponentBeginOverlap` OtherActor) :!label _label))
  (if true
    (set `/Game/V3/Modelos_OBJ/Personaje/Base/BP_gatoBase/Character_gatoBase.vida` (+ (`/Game/V3/Modelos_OBJ/Personaje/Base/BP_gatoBase/Character_gatoBase.vida` _ascharacter_gato_base) 10.0) _ascharacter_gato_base)
    (`KismetSystemLibrary.PrintString` "Eentro")
    (set `self.vida_tomada_cor` true)
    (`GameplayStatics.PlaySound2D` "/Game/V3/SonidosyMusica/Sonidos/power_up.power_up" 1.0 1.0 0.0 null null)
    (`self.K2_DestroyActor`)))

(event `self.Sphere.OnComponentBeginOverlap`
  (params (OverlappedComponent :type "PrimitiveComponent Object Reference") (OtherActor :type "Actor Object Reference") (OtherComp :type "PrimitiveComponent Object Reference") (OtherBodyIndex :type Integer) (bFromSweep :type Boolean) (SweepResult :type "HitResult Structure (by ref)"))
  (goto _label))

(fn `UserConstructionScript`)